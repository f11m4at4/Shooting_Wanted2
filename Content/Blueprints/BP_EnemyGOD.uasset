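; BP_EnemyGOD is an enemy spawner actor that periodically creates an enemy from its EnemyFactory class at its own location.
; Tick accumulates elapsed time and spawns when it exceeds CreateTime, then resets the timer.
; The GetCreateTime helper picks a new random interval between MinTime and MaxTime at BeginPlay and after each spawn.
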(event EventBeginPlay
  (Variables|Default|SetCreateTime (CallFunction|GetCreateTime (Variables|Default|GetMinTime) (Variables|Default|GetMaxTime))))

(event Collision|EventActorBeginOverlap
  (params (OtherActor :type Actor%20Object%20Reference)))

(event EventTick
  (params (DeltaSeconds :type Float%20%28single-precision%29))
  ;[0.15 0.15 0.15 0.5] 시간이 흘러야한다.
  (Variables|Default|SetCurrentTime (+ DeltaSeconds (Variables|Default|GetCurrentTime)))
  ;[0.15 0.15 0.15 0.5] 생성시간이 됐다면
  (if (> (Variables|Default|GetCurrentTime) (Variables|Default|GetCreateTime))
    ;[0.15 0.15 0.15 0.5] 적공장에서 적을 만들고 싶다.
    (Game|SpawnActorfromClass (Variables|Default|GetEnemyFactory) (Math|Transform|MakeTransform (Transformation|GetActorLocation) "0, 0, 0" "1.000000,1.000000,1.000000") "Undefined" "MultiplyWithRoot" 0 0)
    ;[0.15 0.15 0.15 0.5] 경과시간 초기화
    (Variables|Default|SetCurrentTime 0.0)
    (Variables|Default|SetCreateTime (CallFunction|GetCreateTime (Variables|Default|GetMinTime) (Variables|Default|GetMaxTime)))))

(fn ConstructionScript)

(fn GetCreateTime
  (params (Min :type Float%20%28double-precision%29) (Max :type Float%20%28double-precision%29))
  (return (Math|Random|RandomFloatinRange Min Max)))