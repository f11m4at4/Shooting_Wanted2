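; BP_Enemy is an enemy actor that flies in a straight line and explodes on overlap.
; At BeginPlay, FindDirection aims it at BP_Player once, falling back to straight down; the ToTarget random roll currently always passes.
; Tick moves it with a swept offset, and a timer destroys it after DestroyTime.
; Box overlap destroys both actors and plays explosion sound and particles.
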(event OnComponentBeginOverlap(Box)
  (params (OverlappedComponent :type Primitive%20Component%20Object%20Reference) (OtherActor :type Actor%20Object%20Reference) (OtherComp :type Primitive%20Component%20Object%20Reference) (OtherBodyIndex :type Integer) (bFromSweep :type Boolean) (SweepResult :type Hit%20Result%20Structure%20%28by%20ref%29))
  ;[0.15 0.15 0.15 0.5] 부딪혔을 때 처리
  (Actor|DestroyActor OtherActor)
  (Actor|DestroyActor)
  (Audio|PlaySound2D "/Game/Explosion.Explosion" 1.0 1.0 0.0 0 0)
  (Effects|SpawnEmitteratLocation "/Game/StarterContent/Particles/P_Explosion.P_Explosion" (Transformation|GetActorLocation)))

(event Custom|DestroyEvent
  (Actor|DestroyActor))

(event EventBeginPlay
  ;[0.15 0.15 0.15 0.5] 태어나면 방향찾기
  (bind _returnvalue (Actor|GetActorOfClass "/Game/Blueprints/BP_Player.BP_Player_C"))
  (Variables|Default|SetTarget _returnvalue)
  (CallFunction|FindDirection)
  ;[0.15 0.15 0.15 0.5] 죽을 시간 설정
  (Utilities|Time|SetTimerbyEvent (delegate Custom|DestroyEvent) (Variables|Default|GetDestroyTime)))

(event EventTick
  (params (DeltaSeconds :type Float%20%28single-precision%29))
  ;[0.15 0.15 0.15 0.5] 이동하고 싶다.
  ;;[0.15 0.15 0.15 0.5] P
  (Transformation|SetActorLocation (+ (* DeltaSeconds (* (Variables|Default|GetSpeed) (Variables|Default|GetDirection))) (Transformation|GetActorLocation)) true false))

(fn ConstructionScript)

(fn FindDirection
  ;[0.15 0.15 0.15 0.5] 타겟이 있는지 여부 조사
  (Utilities|IsValid (Variables|Default|GetTarget)
    (:Is%20Valid
      ;[0.15 0.15 0.15 0.5] 타겟쪽으로 설정할지 조사
      (if (CallFunction|ToTarget)
        ;[0.15 0.15 0.15 0.5] 타겟으로 향하는 방향구하기
        (Variables|Default|SetDirection (Math|Vector|Normalize (- (Transformation|GetActorLocation (Variables|Default|GetTarget)) (Transformation|GetActorLocation))))
        (else
          (Variables|Default|SetDirection "0.000000,0.000000,-1.000000"))))
    (:Is%20Not%20Valid
      (Variables|Default|SetDirection "0.000000,0.000000,-1.000000")))
  (Transformation|SetActorRotation (Math|Rotator|MakeRotfromXZ (Transformation|GetActorForwardVector) (Variables|Default|GetDirection))))

(fn ToTarget
  (return (<= (Math|Random|RandomIntegerinRange 1 100) 100)))