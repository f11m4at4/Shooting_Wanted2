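; Game mode for a shooter that runs the game flow as an enum state machine through Main Menu, Ready, Playing and Gameover.
; Tick prints the state, lazily creates the main menu widget, and times the Ready delay before setting Playing and hiding the ready UI.
; ChangeState switches from the initial UI-only cursor input to game-only on Ready and notifies the UI on Gameover.
; IsPlaying exposes whether play is active.
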(event EventBeginPlay
  (bind _returnvalue (Game|GetPlayerController 0))
  (Variables|/Script/Engine.PlayerController|SetbShowMouseCursor _returnvalue true)
  (Input|SetInputModeUIOnly _returnvalue 0 "DoNotLock" false))

(event EventTick
  (params (DeltaSeconds :type Float%20%28single-precision%29))
  (bind _state (Variables|Default|GetState))
  (Development|PrintString (Utilities|String|EnumtoString _state))
  (switch Utilities|FlowControl|Switch|SwitchonE_GameState _state
    (:NewEnumerator0
      (CallFunction|MainMenuState))
    (:NewEnumerator1
      (CallFunction|ReadyState))))

(fn ConstructionScript)

(fn MainMenuState
  ;[0.15 0.15 0.15 0.5] ui 가 없다면
  (Utilities|IsValid (Variables|Default|GetMainUI)
    (:Is%20Not%20Valid
      ;[0.15 0.15 0.15 0.5] 생성하고
      (bind _returnvalue (UserInterface|CreateWidget "/Game/UI/WBP_MainMenu.WBP_MainMenu_C"))
      (bind _output_get (Variables|Default|SetMainUI _returnvalue))
      ;[0.15 0.15 0.15 0.5] 화면에 띄워주자
      (UserInterface|Viewport|AddtoViewport _output_get 0))))

(fn ReadyState
  (bind _output_get (Variables|Default|SetCurrentTime (+ (Variables|Default|GetCurrentTime) (Utilities|Time|GetWorldDeltaSeconds))))
  (if (> _output_get (Variables|Default|GetReadyDelayTime))
    (Variables|Default|SetState "NewEnumerator2")
    (Default|OnReadyInvisible (Variables|Default|GetMainUI))))

(fn ChangeState
  (params (NewState :type E_GameState%20Enum :default "NewEnumerator0"))
  (bind _returnvalue (Game|GetPlayerController 0))
  (bind _output_get (Variables|Default|SetState NewState))
  (switch Utilities|FlowControl|Switch|SwitchonE_GameState _output_get
    (:NewEnumerator1
      (Variables|/Script/Engine.PlayerController|SetbShowMouseCursor _returnvalue false)
      (Input|SetInputModeGameOnly _returnvalue false))
    (:NewEnumerator3
      (Default|OnPlayerDie (Variables|Default|GetMainUI)))))

(fn IsPlaying
  (return (Utilities|Enum|Equal(Enum) (Variables|Default|GetState) "NewEnumerator2")))