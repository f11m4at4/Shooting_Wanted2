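; BP_EnemyBoss is an enemy boss that fires a one-time radial burst of BP_EnemyBullet actors when play begins.
; BeginPlay calls MakeBullet once per BulletCount, which spaces bullets by an integer angle step around a circle of radius R.
; Cosine and sine place each bullet in the YZ plane around the boss, and MakeRotFromZ points its Z axis outward from the center.
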(event EventBeginPlay
  (for _index (range 0 (- (Variables|Default|GetBulletCount) 1))
    (CallFunction|MakeBullet _index)))

(fn ConstructionScript)

(fn MakeBullet
  (params (Index :type Integer))
  ;[0.15 0.15 0.15 0.5] 각도를 구한다.
  (Variables|Default|SetAngle (* Index (/ 360 (Variables|Default|GetBulletCount))))
  (LocalVariables|SetY (* (Variables|Default|GetR) (Math|Trig|Cos(Degrees) (Math|Conversions|ToFloat(Integer) (Variables|Default|GetAngle)))))
  (LocalVariables|SetZ (* (Variables|Default|GetR) (Math|Trig|Sin(Degrees) (Math|Conversions|ToFloat(Integer) (Variables|Default|GetAngle)))))
  (bind _output_get (LocalVariables|SetBulletPosition (Math|Vector|MakeVector 0.0 (LocalVariables|GetY) (LocalVariables|GetZ))))
  (Game|SpawnActorfromClass "/Game/Blueprints/BP_EnemyBullet.BP_EnemyBullet_C" (Math|Transform|MakeTransform (+ _output_get (Transformation|GetActorLocation)) (Math|Rotator|MakeRotfromZ (LocalVariables|GetBulletPosition)) "1.000000,1.000000,1.000000") "Undefined" "MultiplyWithRoot" 0 0))