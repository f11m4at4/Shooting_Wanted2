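; BP_Boss is a boss actor that fires BP_EnemyBullet in a circular pattern when play begins.
; OnceFire selects a full ring at once, or a looping ScrewBullet timer that fires one bullet per tick until BulletNumber × ScrewNumber shots clear it.
; FireBullets uses sine and cosine to place each bullet around the boss in the YZ plane, with its Z axis pointing outward.
; Tick is empty, and GetCreateTime is never called here.
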(event EventBeginPlay
  (Variables|Default|SetAngle (/ 360 (Variables|Default|GetBulletNumber)))
  (if (Variables|Default|GetbOnceFire)
    (for _index (range 0 (- (Variables|Default|GetBulletNumber) 0))
      (CallFunction|FireBullets _index))
    (else
      (bind _returnvalue (Utilities|Time|SetTimerbyFunctionName 0 "ScrewBullet" (Variables|Default|GetScrewTime) true))
      (Variables|Default|SetBulletTimer _returnvalue))))

(event Collision|EventActorBeginOverlap
  (params (OtherActor :type Actor%20Object%20Reference)))

(event EventTick
  (params (DeltaSeconds :type Float%20%28single-precision%29)))

(fn ConstructionScript)

(fn GetCreateTime
  (params (Min :type Float%20%28double-precision%29) (Max :type Float%20%28double-precision%29))
  (return (Math|Random|RandomFloatinRange Min Max)))

(fn FireBullets
  (params (A :type Integer))
  (bind _angle (Variables|Default|GetAngle))
  (bind _distance (Variables|Default|GetDistance))
  (bind _returnvalue (* A _angle))
  (bind _returnvalue_2 (Math|Conversions|ToFloat(Integer) _returnvalue))
  (Variables|Default|SetPosition (Math|Vector|MakeVector 0.0 (* (Math|Trig|Cos(Degrees) _returnvalue_2) _distance) (* _distance (Math|Trig|Sin(Degrees) _returnvalue_2))))
  (bind _output_get (Variables|Default|SetPosition (+ (Transformation|GetActorLocation) (Variables|Default|GetPosition))))
  (Game|SpawnActorfromClass "/Game/Blueprints/BP_EnemyBullet.BP_EnemyBullet_C" (Math|Transform|MakeTransform _output_get (Math|Rotator|MakeRotfromZ (- _output_get (Transformation|GetActorLocation))) "1.000000,1.000000,1.000000") "Undefined" "MultiplyWithRoot" 0 0))

(fn ScrewBullet
  (CallFunction|FireBullets (Variables|Default|GetCount))
  (bind _result (Math|Integer|IncrementInt (Variables|Default|GetCount))
    (:%20%20
      (if (>= _result (* (Variables|Default|GetBulletNumber) (Variables|Default|GetScrewNumber)))
        (Utilities|Time|ClearandInvalidateTimerbyHandle (Variables|Default|GetBulletTimer))))))